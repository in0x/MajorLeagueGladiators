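; CloseEnough is a behavior tree decorator that checks whether an enemy AI's pawn is near the actor it is set to follow.
; It casts the owning controller to Enemy_AI_CON and stores that reference.
; It then reads the TargetToFollow actor from the blackboard and passes when the straight-line 3D distance to the pawn is within AcceptableDistance.
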(fn `PerformConditionCheckAI`
  (params (OwnerController :type "AIController Object Reference") (ControlledPawn :type "Pawn Object Reference"))
  (returns (ReturnValue :type Boolean))
  (bind _asenemy_ai_con (cast `/Game/BluePrints/AI/Enemy_AI_CON` OwnerController))
  (set `self.AI_CON_Ref` _asenemy_ai_con)
  (return (<= (`KismetMathLibrary.VSize` (- (`Actor.K2_GetActorLocation` (`BTFunctionLibrary.GetBlackboardValueAsActor` (`self.TargetToFollow`))) (`Actor.K2_GetActorLocation` ControlledPawn))) (`self.AcceptableDistance`))))