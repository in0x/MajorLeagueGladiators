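; Menu actor that shows the player's friends list through a FriendlistWidgetBP hosted in a WidgetComponent.
; When friend data loads from the network, it reuses pooled friend widgets, adds scrollable entries when more are needed, then hides unused ones.
; SetupFriendWidget applies index, username, online state and joinability, and binds and pools new widgets.
; The reuse path calls SetupFriendWidget without passing the friend's State.
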(event `self.ReceiveBeginPlay`
  (cast `/Game/BluePrints/Menu/FriendlistWidgetBP` (`WidgetComponent.GetUserWidgetObject` (`self.widgetComponent`))
    (:`CastFailed`
      (`KismetSystemLibrary.PrintString` "Failed to cast UserWidgetObject to FriendlistWidgetBP"))))

(event `self.OnFriendsInfoLoaded`
  (params (friends :type "Array of FriendState Structure (by ref)"))
  ;[1 1 1] Set up Friends Widgets once loaded from network
  (`KismetSystemLibrary.PrintString` "Setting up Friend Widgets")
  (`|CreateWidget` "/Game/BluePrints/Menu/FriendWidgetBP.FriendWidgetBP_C")
  (bind _asfriendlist_widget_bp (cast `/Game/BluePrints/Menu/FriendlistWidgetBP` (`WidgetComponent.GetUserWidgetObject` (`self.widgetComponent`)))
    (:`then`
      (for (_array_element _array_index) friends
        ;[1 1 1] Update Widget Values (And create new one if more are needed)
        (if (< _array_index (`KismetArrayLibrary.Array_Length` (`self.friendWidgets`)))
          (bind _asfriend_widget_bp (cast `/Game/BluePrints/Menu/FriendWidgetBP` (`|GetArrayItem` (`self.friendWidgets`) _array_index))
            (:`then`
              (`Widget.SetVisibility` _asfriend_widget_bp "Visible")
              (`self.SetupFriendWidget` _asfriend_widget_bp (struct) false))
            (:`CastFailed`
              (`KismetSystemLibrary.PrintString` "Can't cast FriendWidget back to Blueprint Type")))
          (else
            (bind _widget (`/Game/BluePrints/Menu/FriendlistWidgetBP.AddScrollableChild` _asfriendlist_widget_bp))
            (`self.SetupFriendWidget` _widget _array_element true))))
      (`self.HideUnusedWidgets` _array_index))
    (:`CastFailed`
      (`KismetSystemLibrary.PrintString` "Failed to get Friendlist while creating Friendwidgets"))))

(fn `SetupFriendWidget`
  (params (Widget :type "/Game/BluePrints/Menu/FriendWidgetBP Object Reference") (State :type "FriendState Structure") (bIsNewWidget :type Boolean))
  (bind (_username _friendindex _onlinestate _bcanjoin) (break `FriendState` State))
  (`FriendWidget.ChangeFriendIndex` Widget _friendindex)
  (`FriendWidget.ChangeUsername` Widget _username)
  (`FriendWidget.ChangeOnlineState` Widget _onlinestate)
  (`FriendWidget.ChangeCanJoin` Widget _bcanjoin)
  (if bIsNewWidget
    (`self.BindToFriendWidget` Widget)
    (`KismetArrayLibrary.Array_Add` (`self.friendWidgets`) Widget)))

(fn `UserConstructionScript`)