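; EQS context that supplies an AI querier with the closest usable item, either a health pack or an ammo pack.
; ProvideSingleActor adds every HealthPackBP and AmmoPackBP actor to PackSet, then loops over them and returns the nearest to the querier by squared distance.
; PackSet, ClosestPack and ClosestPackDistance are not cleared or reset within the function.
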(fn `ProvideSingleActor`
  (params (QuerierObject :type "Object Object Reference") (QuerierActor :type "Actor Object Reference"))
  (returns (ResultingActor :type "Actor Object Reference"))
  (locals (ClosestPack :type "Actor Object Reference") (ClosestPackDistance :type "Float (double-precision)" :default 3.4028234663852886e+38) (PackSet :type "Set of Actor Object Reference"))
  (bind _packset (`local.PackSet`))
  (bind _outactors (`GameplayStatics.GetAllActorsOfClass` "/Game/BluePrints/HealthPackBP.HealthPackBP_C"))
  (`BlueprintSetLibrary.Set_AddItems` _packset _outactors)
  (bind _outactors_2 (`GameplayStatics.GetAllActorsOfClass` "/Game/BluePrints/AmmoPackBP.AmmoPackBP_C"))
  (`BlueprintSetLibrary.Set_AddItems` _packset _outactors_2)
  (bind _result (`BlueprintSetLibrary.Set_ToArray` _packset))
  (for _array_element _result
    (bind _returnvalue (`KismetMathLibrary.VSizeSquared` (- (`Actor.K2_GetActorLocation` _array_element) (`Actor.K2_GetActorLocation` QuerierActor))))
    (if (< _returnvalue (`local.ClosestPackDistance`))
      (set `local.ClosestPack` _array_element)
      (set `local.ClosestPackDistance` _returnvalue)))
  (return (`local.ClosestPack`)))