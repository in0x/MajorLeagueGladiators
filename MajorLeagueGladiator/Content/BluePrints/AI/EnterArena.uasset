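; Behavior tree task that sends an AI pawn into the arena, using the nearest NavModifierVolume as its reference point.
; On execute it scans all such volumes, keeping the closest by squared distance.
; It then moves the pawn 500 units beyond that volume's center along the approach direction, at the pawn's own height.
; Success sets the HasEntered blackboard key and finishes the task; a failed move fails it.
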(event `self.ReceiveExecuteAI`
  (params (OwnerController :type "AIController Object Reference") (ControlledPawn :type "Pawn Object Reference"))
  (bind _returnvalue (`Actor.K2_GetActorLocation` ControlledPawn))
  (bind _returnvalue_2 (`KismetMathLibrary.MakeVector` (.x (`Actor.K2_GetActorLocation` (`self.ClosestNavModifier`))) (.y (`Actor.K2_GetActorLocation` (`self.ClosestNavModifier`))) (.z _returnvalue)))
  (bind _outactors (`GameplayStatics.GetAllActorsOfClass` "/Script/Engine.NavModifierVolume"))
  (for (_array_element _array_index) _outactors
    (if (== _array_index 0)
      (set `self.ClosestNavModifier` _array_element :!label _label)
      (bind _returnvalue_3 (`KismetMathLibrary.VSizeSquared` (- (`Actor.K2_GetActorLocation` _array_element) _returnvalue)))
      (set `self.ClosestDistance` _returnvalue_3)
      (elif (< _returnvalue_3 (`self.ClosestDistance`))
        (goto _label))))
  (`|AIMoveTo` ControlledPawn (+ _returnvalue_2 (* (`KismetMathLibrary.Normal` (- _returnvalue_2 _returnvalue)) 500)) null 100.0 true
    (:`OnSuccess`
      (`BTFunctionLibrary.SetBlackboardValueAsBool` (`self.HasEntered`) true)
      (`self.FinishExecute` true))
    (:`OnFail`
      (`self.FinishExecute` false))))