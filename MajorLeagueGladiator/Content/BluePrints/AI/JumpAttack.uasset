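; JumpAttack is a Behavior Tree task that triggers the attack of a melee AI character.
; On execute it casts the pawn to MeleeAI_Character, calls OnAttackEvent, then finishes successfully after a fixed delay, without checking the attack's outcome.
; A failed cast stops without finishing the task.
; Tick is empty, and leftover pitch-rotation swing logic is disconnected and never runs.
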(event `self.ReceiveExecuteAI`
  (params (OwnerController :type "AIController Object Reference") (ControlledPawn :type "Pawn Object Reference"))
  (bind _asmelee_ai_character (cast `/Game/BluePrints/AI/MeleeAI_Character` ControlledPawn))
  (`/Game/BluePrints/AI/MeleeAI_Character.OnAttackEvent` _asmelee_ai_character)
  (`GameplayTask_WaitDelay.TaskWaitDelay` OwnerController 3.0
    (:`OnFinish`
      (`self.FinishExecute` true))))

(event `self.ReceiveTickAI`
  (params (OwnerController :type "AIController Object Reference") (ControlledPawn :type "Pawn Object Reference") (DeltaSeconds :type "Float (single-precision)")))