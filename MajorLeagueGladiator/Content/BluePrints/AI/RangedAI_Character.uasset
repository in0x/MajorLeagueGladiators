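; Ranged enemy AI character Blueprint that handles stagger and attack events.
; Stagger stops the AI controller's brain logic on the authority and passes the duration to RangedEnemyAnimBP, while UnStagger restarts that logic, also authority-only.
; Attack forwards its duration to the same animation Blueprint, with no attack logic in this graph.
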(event `self.ReceiveBeginPlay`
  (`parent.ReceiveBeginPlay`))

(event `self.UnStagger`
  (`/Engine/EditorBlueprintResources/ActorMacros.Switch Has Authority`
    (:`Authority`
      (bind _returnvalue (`AIBlueprintHelperLibrary.GetAIController` self))
      (`BrainComponent.RestartLogic` (`AIController.BrainComponent` _returnvalue)))))

(event `self.Stagger`
  (params (Duration :type "Float (single-precision)"))
  (`/Engine/EditorBlueprintResources/ActorMacros.Switch Has Authority`
    (:`Authority`
      (bind _returnvalue (`AIBlueprintHelperLibrary.GetAIController` self))
      (`BrainComponent.StopLogic` (`AIController.BrainComponent` _returnvalue) "Stagger"))
    (:`Remote`
      _))
  (bind _asranged_enemy_anim_bp (cast `/Game/BluePrints/AI/RangedEnemyAnimBP` (`SkeletalMeshComponent.GetAnimInstance` (`self.Mesh`))))
  (`/Game/BluePrints/AI/RangedEnemyAnimBP.OnStaggering` _asranged_enemy_anim_bp Duration))

(event `self.Attack`
  (params (AttackDuration :type "Float (single-precision)"))
  (bind _asranged_enemy_anim_bp (cast `/Game/BluePrints/AI/RangedEnemyAnimBP` (`SkeletalMeshComponent.GetAnimInstance` (`self.Mesh`))))
  (`/Game/BluePrints/AI/RangedEnemyAnimBP.OnAttacking` _asranged_enemy_anim_bp AttackDuration))

(fn `UserConstructionScript`
  (`parent.UserConstructionScript`))