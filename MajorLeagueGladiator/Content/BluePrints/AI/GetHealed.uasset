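; GetHealed is an AI behavior tree task that sends the controlled pawn to the cheapest-to-reach health pack.
; It computes a synchronous navigation path to every HealthPackBP in the level and keeps the one with the lowest path cost, not straight-line distance.
; AIMoveTo then walks the pawn onto it and finishes the task with success or failure, while an abort stops the controller's movement.
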(event `self.ReceiveExecuteAI`
  (params (OwnerController :type "AIController Object Reference") (ControlledPawn :type "Pawn Object Reference"))
  (bind _outactors (`GameplayStatics.GetAllActorsOfClass` "/Game/BluePrints/HealthPackBP.HealthPackBP_C"))
  (for (_array_element _array_index) _outactors
    (bind _returnvalue (`NavigationSystem.FindPathToActorSynchronously` (`Actor.K2_GetActorLocation` ControlledPawn) _array_element 50.0 ControlledPawn))
    (bind _returnvalue_2 (`NavigationPath.GetPathCost` _returnvalue))
    (if (or (== _array_index 0) (< _returnvalue_2 (`self.ShortestPathCost`)))
      (set `self.ClosestPack` _array_element)
      (set `self.ShortestPathCost` _returnvalue_2)))
  (`|AIMoveTo` ControlledPawn (0.0 0.0 0.0) (`self.ClosestPack`) 0.0 true
    (:`OnSuccess`
      (`self.FinishExecute` true))
    (:`OnFail`
      (`self.FinishExecute` false))))

(event `self.ReceiveAbortAI`
  (params (OwnerController :type "AIController Object Reference") (ControlledPawn :type "Pawn Object Reference"))
  (`Controller.StopMovement` OwnerController)
  (`self.FinishAbort`))