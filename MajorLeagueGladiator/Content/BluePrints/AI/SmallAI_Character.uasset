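; Small enemy AI character whose mesh tumbles and bobs in place, extending the behavior of its parent class.
; BeginPlay picks random pitch and yaw spin rates, which Tick applies as delta-time-scaled local rotation.
; Tick also adds a sine-of-elapsed-time vertical world offset to the mesh each frame, not scaled by delta time.
; The Attack event calls OnAggro on the mesh's SmallEnemyAnimBP animation instance.
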(event `self.ReceiveBeginPlay`
  (`parent.ReceiveBeginPlay`)
  (set `self.RotationSpeedY` (`KismetMathLibrary.RandomIntegerInRange` -100 100))
  (set `self.RotationSpeedZ` (`KismetMathLibrary.RandomIntegerInRange` -100 100)))

(event `self.ReceiveTick`
  (params (DeltaSeconds :type "Float (single-precision)"))
  (bind _mesh (`self.Mesh`))
  (`parent.ReceiveTick` DeltaSeconds)
  (`SceneComponent.K2_AddLocalRotation` _mesh (`KismetMathLibrary.MakeRotator` 0.0 (* (`self.RotationSpeedY`) DeltaSeconds) (* (`self.RotationSpeedZ`) DeltaSeconds)) false false)
  (bind _output_get (set `self.TimeSum` (+ DeltaSeconds (`self.TimeSum`))))
  (`SceneComponent.K2_AddWorldOffset` _mesh (`KismetMathLibrary.MakeVector` 0.0 0.0 (* (`KismetMathLibrary.Sin` _output_get) 0.5)) false false))

(event `self.Attack`
  (params (AttackDuration :type "Float (single-precision)"))
  (bind _assmall_enemy_anim_bp (cast `/Game/BluePrints/AI/SmallEnemyAnimBP` (`SkeletalMeshComponent.GetAnimInstance` (`self.Mesh`))))
  (`/Game/BluePrints/AI/SmallEnemyAnimBP.OnAggro` _assmall_enemy_anim_bp))

(fn `UserConstructionScript`
  (`parent.UserConstructionScript`))