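; Behavior Tree task that makes an AI pawn fire a projectile at its blackboard target.
; On execute, it spawns the configured projectile class at a socket on the pawn's skeletal mesh, with the pawn as instigator.
; It launches the projectile's static mesh with a physics impulse along the pawn-to-target direction, scaled by a velocity variable, then immediately finishes successfully.
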(event `self.ReceiveExecuteAI`
  (params (OwnerController :type "AIController Object Reference") (ControlledPawn :type "Pawn Object Reference"))
  (bind _returnvalue (`|SpawnActorFromClass` (`self.Projectile`) (`SceneComponent.GetSocketTransform` (`Actor.GetComponentByClass` ControlledPawn "/Script/Engine.SkeletalMeshComponent") (`self.Socket`) "RTS_World") "Undefined" "OverrideRootScale" null ControlledPawn))
  (`PrimitiveComponent.AddImpulse` (`StaticMeshActor.StaticMeshComponent` _returnvalue) (* (`KismetMathLibrary.Normal` (- (`Actor.K2_GetActorLocation` (`BTFunctionLibrary.GetBlackboardValueAsActor` (`self.Target`))) (`Actor.K2_GetActorLocation` ControlledPawn))) (`self.ProjectileVelocity`)) "None" false)
  (`self.FinishExecute` true))