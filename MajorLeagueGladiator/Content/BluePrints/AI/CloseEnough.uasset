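; CloseEnough is a Behavior Tree decorator that gates AI logic on the pawn's distance from its follow target.
; It reads the TargetToFollow actor from the Blackboard and compares its distance to the controlled pawn against AcceptableDistance.
; Despite the name, it passes when the target is at or beyond that distance, and fails when closer or when the target is invalid.
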(fn `PerformConditionCheckAI`
  (params (OwnerController :type "AIController Object Reference") (ControlledPawn :type "Pawn Object Reference"))
  (returns (ReturnValue :type Boolean))
  (bind _returnvalue (`BTFunctionLibrary.GetBlackboardValueAsActor` (`self.TargetToFollow`)))
  (`/Engine/EditorBlueprintResources/StandardMacros.IsValid` _returnvalue
    (:`Is Valid`
      (return (>= (`KismetMathLibrary.VSize` (- (`Actor.K2_GetActorLocation` _returnvalue) (`Actor.K2_GetActorLocation` ControlledPawn))) (`self.AcceptableDistance`))))
    (:`Is Not Valid`
      (return false))))