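; AggroCheck is a Behavior Tree tick node that picks the nearest target for an enemy AI to attack.
; Each tick resets TargetLocation to a far sentinel, then sphere-traces around the pawn, ignoring all AI_Character actors.
; The closest hit below a world-height limit is written to TargetToAttack and TargetLocation.
; The branch clearing TargetToAttack sits inside the hit loop, so an empty trace leaves the previous target set.
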(event `self.ReceiveTickAI`
  (params (OwnerController :type "AIController Object Reference") (ControlledPawn :type "Pawn Object Reference") (DeltaSeconds :type "Float (single-precision)"))
  (bind _returnvalue (`Actor.K2_GetActorLocation` ControlledPawn))
  (bind _mylocation (`self.MyLocation`))
  (bind _targettoattack (`self.TargetToAttack`))
  (bind _targetlocation (`self.TargetLocation`))
  (if (not (!= (`self.AI_CON_Ref`) null))
    (bind _asenemy_ai_con (cast `/Game/BluePrints/AI/Enemy_AI_CON` OwnerController))
    (set `self.AI_CON_Ref` _asenemy_ai_con))
  (bind _outactors (`GameplayStatics.GetAllActorsOfClass` "/Game/BluePrints/AI/AI_Character.AI_Character_C"))
  (set `self.MyLocation` _returnvalue)
  (`BTFunctionLibrary.SetBlackboardValueAsVector` (`self.TargetLocation`) (100000.0 100000.0 100000.0))
  (bind (_outhits _returnvalue_2) (`KismetSystemLibrary.SphereTraceMultiForObjects` _returnvalue (+ _returnvalue (0.0 0.0 15.0)) 1500.0 (`self.DesiredObjectTypes`) false _outactors))
  (for _array_element _outhits
    (if _returnvalue_2
      (bind (_bblockinghit _binitialoverlap _time _location _impactpoint _normal _impactnormal _physmat _hitactor) (`GameplayStatics.BreakHitResult` _array_element))
      (bind _returnvalue_3 (`Actor.K2_GetActorLocation` _hitactor))
      (if (and (< (.z _returnvalue_3) 300.0) (< (`KismetMathLibrary.VSizeSquared` (- _returnvalue_3 _mylocation)) (`KismetMathLibrary.VSizeSquared` (- (`BTFunctionLibrary.GetBlackboardValueAsVector` _targetlocation) _mylocation))))
        (`BTFunctionLibrary.SetBlackboardValueAsObject` _targettoattack _hitactor)
        (`BTFunctionLibrary.SetBlackboardValueAsVector` _targetlocation _returnvalue_3))
      (else
        (`BTFunctionLibrary.SetBlackboardValueAsObject` _targettoattack)))))