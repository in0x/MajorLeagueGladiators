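; EQS context that supplies the player character nearest to the querier for AI environment queries.
; ProvideSingleActor scans every MlgPlayerCharacter and compares squared distances to the querier's location.
; The running closest player and distance live in variables that the function never resets before the scan.
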(fn `ProvideSingleActor`
  (params (QuerierObject :type "Object Object Reference") (QuerierActor :type "Actor Object Reference"))
  (returns (ResultingActor :type "Actor Object Reference"))
  (locals (ClosestPlayer :type "Actor Object Reference") (ClosestPlayerDistance :type "Float (double-precision)" :default 3.4028234663852886e+38))
  (bind _outactors (`GameplayStatics.GetAllActorsOfClass` "/Script/MajorLeagueGladiator.MlgPlayerCharacter"))
  (for _array_element _outactors
    (bind _returnvalue (`KismetMathLibrary.VSizeSquared` (- (`Actor.K2_GetActorLocation` _array_element) (`Actor.K2_GetActorLocation` QuerierActor))))
    (if (< _returnvalue (`local.ClosestPlayerDistance`))
      (set `local.ClosestPlayer` _array_element)
      (set `local.ClosestPlayerDistance` _returnvalue)))
  (return (`local.ClosestPlayer`)))