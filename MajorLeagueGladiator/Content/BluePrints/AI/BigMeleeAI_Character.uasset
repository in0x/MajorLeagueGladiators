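; Character Blueprint for a big melee AI enemy that forwards combat and health events to its animation Blueprint.
; It binds to the Health component's change delegate on BeginPlay and calls OnStaggering on BigMeleeEnemyAnimBP when health is at or below a quarter, through a handler named CrawlingEvent.
; Attack passes its duration to the same AnimBP, while Stagger and UnStagger are empty.
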(event `self.ReceiveBeginPlay`
  (`parent.ReceiveBeginPlay`)
  (add `HealthComponent.HealthChangedDelegate` (`self.health`) (delegate `CrawlingEvent`)))

(event `CrawlingEvent`
  (params (newHealthPercentage :type "Float (double-precision)") (oldHealthPercentage :type "Float (double-precision)"))
  (if (<= newHealthPercentage 0.25)
    (bind _asbig_melee_enemy_anim_bp (cast `/Game/BluePrints/AI/BigMeleeEnemyAnimBP` (`SkeletalMeshComponent.GetAnimInstance` (`self.Mesh`))))
    (`/Game/BluePrints/AI/BigMeleeEnemyAnimBP.OnStaggering` _asbig_melee_enemy_anim_bp 0.0)))

(event `self.Attack`
  (params (AttackDuration :type "Float (single-precision)"))
  (bind _asbig_melee_enemy_anim_bp (cast `/Game/BluePrints/AI/BigMeleeEnemyAnimBP` (`SkeletalMeshComponent.GetAnimInstance` (`self.Mesh`))))
  (`/Game/BluePrints/AI/BigMeleeEnemyAnimBP.OnAttacking` _asbig_melee_enemy_anim_bp AttackDuration))

(event `self.Stagger`
  (params (Duration :type "Float (single-precision)")))

(event `self.UnStagger`)

(fn `UserConstructionScript`
  (`parent.UserConstructionScript`))